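; BP_GameModeBase is a game mode that hands each player logging in a survivor character already placed in the level.
; On PostLogin, while a switch counter is zero, it caches all BP_SurvivorCharacter actors, then calls SetPlayer and PossessEvent on a random one.
; It then removes a random pick from the pool, evaluated separately from the possessed one, and increments the counter, printing debug messages.
; BeginPlay calls Start.
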(event EventBeginPlay
  (Class|DryFlowerGameModeBase|Start))

(event EventTick
  (params (DeltaSeconds :type Float%20%28single-precision%29)))

(event EventPostLogin
  (params (NewPlayer :type Player%20Controller%20Object%20Reference))
  ;[1 1 1] 클라이언트/ 처음 한 번 실행 : 전체 캐릭터 배열 생성
  (switch int (Variables|Default|GetSwitch)
    (:Default
      _)
    (:0
      (bind _outactors (Actor|GetAllActorsOfClass "/Game/Character/BP/BP_SurvivorCharacter.BP_SurvivorCharacter_C"))
      (bind _output_get (Variables|Default|SetCharacters _outactors))))
  ;[1 1 1] 클라이언트/ 캐릭터 빙의 후 배열 삭제 - 레벨 블프에 있는것과 같은 과정이지만 게임모드에서 실행시켜야 제대로 실행됨
  ;;[1 1 1] 없어도 됨
  (bind _asbp_survivor_character (Utilities|Casting|CastToBP_SurvivorCharacter (.OutItem (Utilities|Array|Random _output_get)))
    (:then
      (Default|SetPlayer _asbp_survivor_character NewPlayer)
      (Default|PossessEvent _asbp_survivor_character)
      (Development|PrintString "Gamemode Possess Succeed")
      (Utilities|Array|RemoveItem _output_get (.OutItem (Utilities|Array|Random _output_get)))
      (Math|Integer|IncrementInt (Variables|Default|GetSwitch)
        (:%20%20
          (for _array_element _output_get
            (Development|PrintString (Utilities|GetDisplayName _array_element))))))
    (:CastFailed
      (Development|PrintString "Gamemode Possess Failed"))))

(fn ConstructionScript)