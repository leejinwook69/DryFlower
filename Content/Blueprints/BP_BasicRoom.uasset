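; BP_BasicRoom is a room actor that places itself on a nine-column grid and builds its own walls, doors and corners.
; SetLocationEvent derives position from RoomNumber and displays RoomType as temporary text, recoloring it for PlayerSpawn.
; AfterInitialEvent adds static mesh components from per-side wall and door flags, with doors mid-wall and columns where walls meet.
; The Construction Script holds an unconnected copy of this build logic, which never runs.
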(event Custom|AfterInitialEvent
  (bind _returnvalue (Math|Rotator|MakeRotator 0.0 0.0 2.7e+02))
  (bind _returnvalue_2 (Math|Rotator|MakeRotator 0.0 0.0 1.8e+02))
  (bind _returnvalue_3 (Math|Rotator|MakeRotator 0.0 0.0 0.0))
  (bind _returnvalue_4 (Math|Rotator|MakeRotator 0.0 0.0 9e+01))
  ;[1 1 1] 데이터 참조하여 상하좌우 벽, 문 생성
  (Utilities|FlowControl|Sequence
    (:then_0
      ;;[1 1 1] 위쪽벽 만들기 시작
      (if (Variables|Default|GettopWall)
        (for _index (range 0 4)
          (if (== _index 2)
            (if (Variables|Default|GettopDoor)
              ;;[1 1 1] 문 만들기
              (bind _returnvalue_5 (AddComponent|AddStaticMeshComponent false (Math|Transform|MakeTransform (- (Math|Vector|MakeVector (* _index 3e+02) -3e+02 0.0) "150.000000, 0, 0") _returnvalue_3 "1,1,1")))
              (Components|StaticMesh|SetStaticMesh _returnvalue_5 "/Game/SciFi_Medical_Room/Meshes/SM_Wall04.SM_Wall04")
              (else
                ;;[1 1 1] 벽 만들기
                (bind _returnvalue_6 (AddComponent|AddStaticMeshComponent false (Math|Transform|MakeTransform (Math|Vector|MakeVector (* _index 3e+02) -3e+02 0.0) _returnvalue_3 "1,1,1") :!label _label))
                (Components|StaticMesh|SetStaticMesh _returnvalue_6 "/Game/SciFi_Medical_Room/Meshes/SM_Wall02.SM_Wall02")))
            (else
              (goto _label))))))
    (:then_1
      ;;[1 1 1] 오른쪽벽 만들기 시작
      (if (Variables|Default|GetrightWall)
        (for _index_2 (range 0 2)
          (if (== _index_2 1)
            (if (Variables|Default|GetrightDoor)
              ;;[1 1 1] 문 만들기
              (bind _returnvalue_7 (AddComponent|AddStaticMeshComponent false (Math|Transform|MakeTransform (- (Math|Vector|MakeVector 1.2e+03 (* _index_2 3e+02) 0.0) "0.000000,150.000000,0.000000") _returnvalue_4 "1,1,1")))
              (Components|StaticMesh|SetStaticMesh _returnvalue_7 "/Game/SciFi_Medical_Room/Meshes/SM_Wall04.SM_Wall04")
              (else
                ;;[1 1 1] 벽 만들기
                (bind _returnvalue_8 (AddComponent|AddStaticMeshComponent false (Math|Transform|MakeTransform (Math|Vector|MakeVector 1.2e+03 (* _index_2 3e+02) 0.0) _returnvalue_4 "1,1,1") :!label _label_2))
                (Components|StaticMesh|SetStaticMesh _returnvalue_8 "/Game/SciFi_Medical_Room/Meshes/SM_Wall02.SM_Wall02")))
            (else
              (goto _label_2))))))
    (:then_2
      ;;[1 1 1] 아래쪽벽 만들기 시작
      (if (Variables|Default|GetbottomWall)
        (for _index_3 (range 0 4)
          (if (== _index_3 2)
            (if (Variables|Default|GetbottomDoor)
              ;;[1 1 1] 문 만들기
              (bind _returnvalue_9 (AddComponent|AddStaticMeshComponent false (Math|Transform|MakeTransform (- (Math|Vector|MakeVector (- 9e+02 (* _index_3 3e+02)) 6e+02 0.0) "-150.000000,0.000000,0.000000") _returnvalue_2 "1,1,1")))
              (Components|StaticMesh|SetStaticMesh _returnvalue_9 "/Game/SciFi_Medical_Room/Meshes/SM_Wall04.SM_Wall04")
              (else
                ;;[1 1 1] 벽 만들기
                (bind _returnvalue_10 (AddComponent|AddStaticMeshComponent false (Math|Transform|MakeTransform (Math|Vector|MakeVector (- 9e+02 (* _index_3 3e+02)) 6e+02 0.0) _returnvalue_2 "1,1,1") :!label _label_3))
                (Components|StaticMesh|SetStaticMesh _returnvalue_10 "/Game/SciFi_Medical_Room/Meshes/SM_Wall02.SM_Wall02")))
            (else
              (goto _label_3))))))
    (:then_3
      ;;[1 1 1] 왼쪽벽 만들기 시작
      (if (Variables|Default|GetleftWall)
        (for _index_4 (range 0 2)
          (if (== _index_4 1)
            (if (Variables|Default|GetleftDoor)
              ;;[1 1 1] 문 만들기
              (bind _returnvalue_11 (AddComponent|AddStaticMeshComponent false (Math|Transform|MakeTransform (- (Math|Vector|MakeVector -3e+02 (- 3e+02 (* _index_4 3e+02)) 0.0) "0.000000,-150.000000,0.000000") _returnvalue "1,1,1")))
              (Components|StaticMesh|SetStaticMesh _returnvalue_11 "/Game/SciFi_Medical_Room/Meshes/SM_Wall04.SM_Wall04")
              (else
                ;;[1 1 1] 벽 만들기
                (bind _returnvalue_12 (AddComponent|AddStaticMeshComponent false (Math|Transform|MakeTransform (Math|Vector|MakeVector -3e+02 (- 3e+02 (* _index_4 3e+02)) 0.0) _returnvalue "1,1,1") :!label _label_4))
                (Components|StaticMesh|SetStaticMesh _returnvalue_12 "/Game/SciFi_Medical_Room/Meshes/SM_Wall02.SM_Wall02")))
            (else
              (goto _label_4))))))
    (:then_4
      ;;[1 1 1] 왼쪽위 모서리 만들기
      (if (and (Variables|Default|GettopWall) (Variables|Default|GetleftWall))
        (bind _returnvalue_13 (AddComponent|AddStaticMeshComponent false (Math|Transform|MakeTransform "-300.000000,-300.000000, 0" "0, 0, 0" "1,1,1")))
        (Components|StaticMesh|SetStaticMesh _returnvalue_13 "/Game/SciFi_Medical_Room/Meshes/SM_Column.SM_Column")))
    (:then_5
      ;;[1 1 1] 오른쪽위 모서리 만들기
      (if (and (Variables|Default|GettopWall) (Variables|Default|GetrightWall))
        (bind _returnvalue_14 (AddComponent|AddStaticMeshComponent false (Math|Transform|MakeTransform "1200.000000,-300.000000, 0" "0,90.000000, 0" "1,1,1")))
        (Components|StaticMesh|SetStaticMesh _returnvalue_14 "/Game/SciFi_Medical_Room/Meshes/SM_Column.SM_Column")))
    (:then_6
      ;;[1 1 1] 오른쪽아래 모서리 만들기
      (if (and (Variables|Default|GetbottomWall) (Variables|Default|GetrightWall))
        (bind _returnvalue_15 (AddComponent|AddStaticMeshComponent false (Math|Transform|MakeTransform "1200.000000,600.000000, 0" "0,180.000000, 0" "1,1,1")))
        (Components|StaticMesh|SetStaticMesh _returnvalue_15 "/Game/SciFi_Medical_Room/Meshes/SM_Column.SM_Column")))
    (:then_7
      ;;[1 1 1] 왼쪽아래 모서리 만들기
      (if (and (Variables|Default|GetbottomWall) (Variables|Default|GetleftWall))
        (bind _returnvalue_16 (AddComponent|AddStaticMeshComponent false (Math|Transform|MakeTransform "-300.000000,600.000000, 0" "0,270.000000, 0" "1,1,1")))
        (Components|StaticMesh|SetStaticMesh _returnvalue_16 "/Game/SciFi_Medical_Room/Meshes/SM_Column.SM_Column")))))

(event Custom|SetLocationEvent
  (bind _roomnumber (Variables|Default|GetroomNumber))
  (bind _roomtype (Variables|Default|GetroomType))
  (bind _textrender (Variables|Default|GetTextRender))
  (bind _returnvalue (Utilities|String|EnumtoString _roomtype))
  ;[1 1 1] RoomNumber를 사용하여 방 위치 선정
  (Transformation|SetActorLocation (Math|Vector|MakeVector (* (Math|Integer|%(Integer) _roomnumber 9) 1.5e+03) (* (/ _roomnumber 9) 9e+02) 0.0) false false)
  ;[1 1 1] RoomType을 사용하여 방에 임시 텍스트 출력
  (Rendering|Components|TextRender|SetText _textrender (Utilities|Text|ToText(String) _returnvalue))
  (if (Utilities|Enum|Equal(Enum) _returnvalue "PlayerSpawn")
    (Rendering|Components|TextRender|SetTextRenderColor _textrender (Math|Color|MakeColor 0 0 255 0))))

(fn ConstructionScript
  ;[1 1 1] 데이터 참조하여 상하좌우 벽, 문 생성
)