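; BP_MurdererCharacter3 is a murderer character Blueprint that handles a melee attack and possession by its Player reference.
; Start and end attack events toggle IsAttacking to block attack spamming, while the hit-check event sphere-traces forward for pawns and applies damage at the moment of impact.
; An older right-hand capsule overlap approach remains unconnected, and SetPlayer is empty.
; Possess_Event makes Player possess this character.
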(event OnComponentBeginOverlap(Capsule)
  (params (OverlappedComponent :type Primitive%20Component%20Object%20Reference) (OtherActor :type Actor%20Object%20Reference) (OtherComp :type Primitive%20Component%20Object%20Reference) (OtherBodyIndex :type Integer) (bFromSweep :type Boolean) (SweepResult :type Hit%20Result%20Structure%20%28by%20ref%29))
  ;[1 1 1] 콜리전 오른손에 붙여서 데미지 주기
)

(event Custom|SetPlayer
  (params (Player :type Player%20Controller%20Object%20Reference))
  ;[1 1 1] 빙의할 플레이어 설정
)

(event Custom|Possess_Event
  ;[1 1 1] 폰 빙의 이벤트
  (Pawn|Possess (stale Custom|SetPlayer Player) self))

(event Custom|OnCollCheck_Attack
  (bind _returnvalue (Transformation|GetActorLocation))
  ;[1 1 1] 타격 순간만 콜리전 만들어서 데미지 주기
  (bind (_outhits _returnvalue_2) (Collision|MultiSphereTraceForObjects _returnvalue (+ _returnvalue (* (Math|Vector|GetForwardVector (Variables|Default|GetCapsuleComponent)) (Variables|Default|GetAtkRange))) 6e+01 (Utilities|Array|MakeArray "ObjectTypeQuery3") false 0 "None"))
  (if _returnvalue_2
    (for _array_element _outhits
      (Game|Damage|ApplyDamage (.HitActor (Collision|BreakHitResult _array_element)) (Variables|Default|GetAtkDamage) 0 self))))

(event Custom|Start_Attack
  ;[1 1 1] 연타 방지
  (Variables|Default|SetIsAttacking true))

(event Custom|End_Attack
  ;[1 1 1] 연타 방지
  (Variables|Default|SetIsAttacking false))

(event Custom|OnCollEnd_Attack
  ;[1 1 1] 콜리전 오른손에 붙여서 데미지 주기
)

(event Custom|OnCollStart_Attack
  ;[1 1 1] 콜리전 오른손에 붙여서 데미지 주기
)

(event EventBeginPlay)

(event Collision|EventActorBeginOverlap
  (params (OtherActor :type Actor%20Object%20Reference)))

(event EventTick
  (params (DeltaSeconds :type Float%20%28single-precision%29)))

(fn ConstructionScript)