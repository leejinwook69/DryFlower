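; BP_SurvivorCharacter is the survivor character Blueprint, handling damage, a key-triggered death and possession.
; Pressing G calls Die, shrinks the capsule to zero size, then calls CallPossess; neither Die nor CallPossess is defined here.
; AnyDamage subtracts from HP, but its zero-HP check leads to no action.
; Possess_Event makes player controller 0 possess this character, while BeginPlay, overlap and Tick are empty.
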(event Custom|Possess_Event
  ;[1 1 1] 폰 빙의 이벤트
  (Pawn|Possess (Game|GetPlayerController 0) self))

(event EventBeginPlay)

(event Collision|EventActorBeginOverlap
  (params (OtherActor :type Actor%20Object%20Reference)))

(event EventTick
  (params (DeltaSeconds :type Float%20%28single-precision%29)))

(event Game|Damage|EventAnyDamage
  (params (Damage :type Float%20%28single-precision%29) (DamageType :type Damage%20Type%20Object%20Reference) (InstigatedBy :type Controller%20Object%20Reference) (DamageCauser :type Actor%20Object%20Reference))
  (bind _output_get (Variables|Default|SetHP (- (Variables|Default|GetHP) Damage)))
  (if (<= _output_get 0.0)
    _))

(event Input|KeyboardEvents|G
  (params (Key :type Key%20Structure :default "None"))
  (:Pressed
    (Class|MyCharacter|Die)
    (Components|Capsule|SetCapsuleSize (Variables|Default|GetCapsuleComponent) 0.0 0.0 false)
    (Default|CallPossess)))

(fn ConstructionScript)