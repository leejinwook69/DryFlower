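; BP_OnlyBPDoorTest is a Blueprint-only test door that slides its StaticMesh along local Z while something overlaps its Cube trigger.
; Cube begin and end overlap set and clear NeedOpen, with no filter on the overlapping actor.
; Tick offsets the mesh by MoveSpd scaled by delta time, reversing it when NeedOpen is false.
; MinLocation and MaxLocation gate the movement by relative Z, without clamping overshoot.
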(event OnComponentBeginOverlap(Cube)
  (params (OverlappedComponent :type Primitive%20Component%20Object%20Reference) (OtherActor :type Actor%20Object%20Reference) (OtherComp :type Primitive%20Component%20Object%20Reference) (OtherBodyIndex :type Integer) (bFromSweep :type Boolean) (SweepResult :type Hit%20Result%20Structure%20%28by%20ref%29))
  (Variables|Default|SetNeedOpen true))

(event OnComponentEndOverlap(Cube)
  (params (OverlappedComponent :type Primitive%20Component%20Object%20Reference) (OtherActor :type Actor%20Object%20Reference) (OtherComp :type Primitive%20Component%20Object%20Reference) (OtherBodyIndex :type Integer))
  (Variables|Default|SetNeedOpen false))

(event EventBeginPlay)

(event Collision|EventActorBeginOverlap
  (params (OtherActor :type Actor%20Object%20Reference)))

(event EventTick
  (params (DeltaSeconds :type Float%20%28single-precision%29))
  (bind _staticmesh (Variables|Default|GetStaticMesh))
  (bind _movespd (Variables|Default|GetMoveSpd))
  (bind _staticmesh_2 (Variables|Default|GetStaticMesh))
  (bind _returnvalue (* DeltaSeconds _movespd))
  (bind _relativelocation (Variables|/Script/Engine.SceneComponent|GetRelativeLocation _staticmesh_2))
  (bind _z (Math|Vector|BreakVector _relativelocation))
  (if (Variables|Default|GetNeedOpen)
    (if (<= (Variables|Default|GetMinLocation) _z)
      (Transformation|AddLocalOffset _staticmesh (Math|Vector|MakeVector 0.0 0.0 _returnvalue) false false))
    (elif (<= _z (Variables|Default|GetMaxLocation))
      (Transformation|AddLocalOffset _staticmesh (Math|Vector|MakeVector 0.0 0.0 (* _returnvalue -1.0)) false false))))

(fn ConstructionScript)